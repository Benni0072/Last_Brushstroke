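; BP_Kiste is an interactable chest puzzle with three number wheels (Zahlenrad), built on a parent that handles interaction and returning to the character.
; BeginPlay gathers the wheels into the Disc array, and SelectedDiscIndex picks the active one.
; Interacting highlights the selected wheel; exiting via IA_ExitPuzzle returns to the character and clears the highlight.
; Left/right navigation inputs and ChangeSelectedDisc are empty stubs, so selection does not change here.
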(event `self.ReceiveBeginPlay`
  (`parent.ReceiveBeginPlay`)
  (set `self.Disc` (`|MakeArray` (`self.BP_Zahlenrad1`) (`self.BP_Zahlenrad2`) (`self.BP_Zahlenrad`))))

(event `self.ReturnToCharacter`
  (`parent.ReturnToCharacter`)
  (`self.SetSelectedDiscHighlight` false))

(event `EnhancedInput|/Game/Inputs/InputActions/IA_ExitPuzzle`
  (params (ActionValue :type Boolean) (ElapsedSeconds :type "Float (double-precision)") (TriggeredSeconds :type "Float (double-precision)") (InputAction :type "InputAction Object Reference" :default "/Game/Inputs/InputActions/IA_ExitPuzzle.IA_ExitPuzzle"))
  (:`Triggered`
    (`self.ReturnToCharacter`)))

(event `EnhancedInput|/Game/Inputs/InputActions/IA_NavigateRight`
  (params (ActionValue :type Boolean) (ElapsedSeconds :type "Float (double-precision)") (TriggeredSeconds :type "Float (double-precision)") (InputAction :type "InputAction Object Reference" :default "/Game/Inputs/InputActions/IA_NavigateRight.IA_NavigateRight")))

(event `EnhancedInput|/Game/Inputs/InputActions/IA_NavigateLeft`
  (params (ActionValue :type Boolean) (ElapsedSeconds :type "Float (double-precision)") (TriggeredSeconds :type "Float (double-precision)") (InputAction :type "InputAction Object Reference" :default "/Game/Inputs/InputActions/IA_NavigateLeft.IA_NavigateLeft")))

(fn `ChangeSelectedDisc`)

(fn `GetSelectedDisc`
  (returns (Output :type "/Game/BPs/Kiste/BP_Zahlenrad Object Reference"))
  (return (`|GetArrayItem` (`self.Disc`) (`self.SelectedDiscIndex`))))

(fn `Interact`
  (params (PlayerCharacter :type "/Game/BPs/BP_FirstPersonCharacter Object Reference") (Pickup :type "/Game/BPs/Pickup/BP_Pickup Object Reference"))
  (returns (UsedUpPickup :type Boolean))
  (`parent.Interact` PlayerCharacter Pickup)
  (`self.SetSelectedDiscHighlight` true)
  (return false))

(fn `SetSelectedDiscHighlight`
  (params (Enable :type Boolean))
  (`self.SetHighlight` Enable (`self.GetSelectedDisc`)))

(fn `UserConstructionScript`)