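; Rotating number wheel (Zahlenrad) that steps between numbered faces, apparently part of a chest or box (Kiste).
; Rotate moves the selected face up or down and derives a target roll from the face count, which Tick eases toward along the shortest path.
; GetCurrentNumber maps the face index to a digit enum in reverse order.
; ClampSelectedFace wraps the index, though underflow lands on NumFaces, one past the last face.
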(event `self.ReceiveTick`
  (params (DeltaSeconds :type "Float (single-precision)"))
  (`self.K2_SetRelativeRotation` (`KismetMathLibrary.RLerp` (`self.RelativeRotation`) (`KismetMathLibrary.MakeRotator` (`self.TargetRot`)) (* (`GameplayStatics.GetWorldDeltaSeconds`) 10.0) true)))

(event `Rotate`
  (params (Up :type Boolean))
  (bind _output_get (set `self.CurrentSelectedFace` (`self.ClampSelectedFace` (+ (`self.CurrentSelectedFace`) (`KismetMathLibrary.SelectInt` 1 -1 Up)))))
  (set `self.TargetRot` (* (`KismetMathLibrary.Conv_IntToDouble` _output_get) (/ 360.0 (`KismetMathLibrary.Conv_IntToDouble` (`self.NumFaces`))) -1.0)))

(fn `ClampSelectedFace`
  (params (Index :type Integer))
  (returns (ReturnVelue :type Integer))
  (locals (ClampeIndex :type Integer))
  (set `local.ClampeIndex` Index)
  (`|ExecutionSequence`
    (:`then_0`
      (if (> (`local.ClampeIndex`) (- (`self.NumFaces`) 1))
        (set `local.ClampeIndex` 0)))
    (:`then_1`
      (if (< (`local.ClampeIndex`) 0)
        (set `local.ClampeIndex` (- (`self.NumFaces`) 0))))
    (:`then_2`
      (return (`local.ClampeIndex`)))))

(fn `GetCurrentNumber`
  (returns (ReturnValue :type "/Game/BPs/Kiste/ERotationLockNumber Enum"))
  (return (select `int` (`self.CurrentSelectedFace`) :`0` "NewEnumerator0" :`1` "NewEnumerator9" :`2` "NewEnumerator8" :`3` "NewEnumerator7" :`4` "NewEnumerator6" :`5` "NewEnumerator5" :`6` "NewEnumerator4" :`7` "NewEnumerator3" :`8` "NewEnumerator2" :`9` "NewEnumerator1" :!type "/Game/BPs/Kiste/ERotationLockNumber Enum")))