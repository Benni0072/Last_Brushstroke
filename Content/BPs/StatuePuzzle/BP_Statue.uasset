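; BP_Statue is a rotatable statue for the statue puzzle that turns in steps between a set number of faces.
; Rotate moves the selected face index up or down without wrapping and converts it into a negated target yaw from the face count.
; Tick eases the relative rotation toward that yaw with a delta-time-scaled, shortest-path lerp.
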(event `self.ReceiveTick`
  (params (DeltaSeconds :type "Float (single-precision)"))
  (`self.K2_SetRelativeRotation` (`KismetMathLibrary.RLerp` (`self.RelativeRotation`) (`KismetMathLibrary.MakeRotator` 0.0 0.0 (`self.TargetRot`)) (* (`GameplayStatics.GetWorldDeltaSeconds`) 10.0) true)))

(event `Rotate`
  (params (Right :type Boolean))
  (bind _output_get (set `self.CurrentSelectedFace` (+ (`self.CurrentSelectedFace`) (`KismetMathLibrary.SelectInt` 1 -1 Right))))
  (set `self.TargetRot` (* (`KismetMathLibrary.Conv_IntToDouble` _output_get) (/ 360.0 (`KismetMathLibrary.Conv_IntToDouble` (`self.NumFaces`))) -1.0)))