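; BP_Chest is a possessable puzzle chest with a three-disc combination lock.
; Interacting shows a controls widget and highlights the selected disc; navigation inputs switch discs and rotate them.
; The interact input checks the discs against CorrectCode: a match blends to a camera, animates latch and lid via timeline, then returns to the character and disables possession.
; A wrong code briefly shows an inspect-text widget, guarded against repeats.
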(event `self.ReceiveBeginPlay`
  (`parent.ReceiveBeginPlay`)
  (set `self.Disc` (`|MakeArray` (`self.BP_Zahlenrad`) (`self.BP_Zahlenrad1`) (`self.BP_Zahlenrad2`))))

(event `self.ReturnToCharacter`
  (`parent.ReturnToCharacter`)
  (`self.SetSelectedDiscHighlight` false)
  (`Widget.RemoveFromParent` (`self.BPW_Painting`)))

(event `EnhancedInput|/Game/Inputs/InputActions/IA_ExitPuzzle`
  (params (ActionValue :type Boolean) (ElapsedSeconds :type "Float (double-precision)") (TriggeredSeconds :type "Float (double-precision)") (InputAction :type "InputAction Object Reference" :default "/Game/Inputs/InputActions/IA_ExitPuzzle.IA_ExitPuzzle"))
  (:`Triggered`
    (`self.ReturnToCharacter`)))

(event `EnhancedInput|/Game/Inputs/InputActions/IA_NavigateRight`
  (params (ActionValue :type Boolean) (ElapsedSeconds :type "Float (double-precision)") (TriggeredSeconds :type "Float (double-precision)") (InputAction :type "InputAction Object Reference" :default "/Game/Inputs/InputActions/IA_NavigateRight.IA_NavigateRight"))
  (:`Triggered`
    (`self.ChangeSelectedDisc` true)))

(event `EnhancedInput|/Game/Inputs/InputActions/IA_NavigateLeft`
  (params (ActionValue :type Boolean) (ElapsedSeconds :type "Float (double-precision)") (TriggeredSeconds :type "Float (double-precision)") (InputAction :type "InputAction Object Reference" :default "/Game/Inputs/InputActions/IA_NavigateLeft.IA_NavigateLeft"))
  (:`Triggered`
    (`self.ChangeSelectedDisc` false)))

(event `EnhancedInput|/Game/Inputs/InputActions/IA_NavigateUp`
  (params (ActionValue :type Boolean) (ElapsedSeconds :type "Float (double-precision)") (TriggeredSeconds :type "Float (double-precision)") (InputAction :type "InputAction Object Reference" :default "/Game/Inputs/InputActions/IA_NavigateUp.IA_NavigateUp"))
  (:`Triggered`
    (`/Game/BPs/Chest/BP_NumberWheel.Rotate` (`self.GetSelectedDisc`) false)))

(event `EnhancedInput|/Game/Inputs/InputActions/IA_NavigateDown`
  (params (ActionValue :type Boolean) (ElapsedSeconds :type "Float (double-precision)") (TriggeredSeconds :type "Float (double-precision)") (InputAction :type "InputAction Object Reference" :default "/Game/Inputs/InputActions/IA_NavigateDown.IA_NavigateDown"))
  (:`Triggered`
    (`/Game/BPs/Chest/BP_NumberWheel.Rotate` (`self.GetSelectedDisc`) true)))

(event `EnhancedInput|/Game/Inputs/InputActions/IA_Interact`
  (params (ActionValue :type Boolean) (ElapsedSeconds :type "Float (double-precision)") (TriggeredSeconds :type "Float (double-precision)") (InputAction :type "InputAction Object Reference" :default "/Game/Inputs/InputActions/IA_Interact.IA_Interact"))
  (:`Triggered`
    (if (`self.EvaluateCombination`)
      (`PlayerController.SetViewTargetWithBlend` (`GameplayStatics.GetPlayerController` 0) (`self.Camera Actor`) (`self.SmoothPossesDuration`) "VTBlend_EaseInOut" (`self.Possess Blend Exp`) false)
      (`KismetSystemLibrary.Delay` (`self.SmoothPossesDuration`))
      (`GameplayStatics.PlaySound2D` "/Game/Sound/SFX/Chest/Lock-002.Lock-002" 1.0 1.0 0.0 null null)
      (bind (_direction _deckel _schnalle) (`Timeline|OpenChest`)
        (:`Update`
          (`SceneComponent.K2_SetRelativeRotation` (`self.Scene`) (`KismetMathLibrary.MakeRotator` (* _schnalle (`self.OpenSchnalleAngle`))) false false)
          (`SceneComponent.K2_SetRelativeRotation` (`self.Scene1`) (`KismetMathLibrary.MakeRotator` (* _deckel (`self.OpenAngle`))) false false)
          (`KismetSystemLibrary.Delay` 2.1)
          (`self.ReturnToCharacter`)
          (set `self.CanBePossessed?` false)))
      (elif (`self.Already Open`)
        (set `self.Already Open` false)
        (bind _returnvalue (`|CreateWidget` "/Game/BPs/InspectableItem/BPW_Inspectable.BPW_Inspectable_C" (`GameplayStatics.GetPlayerController` 0) (`self.Item Text`) (`self.EEmotion`)))
        (bind _output_get (set `self.InspectableWidget` _returnvalue))
        (`UserWidget.AddToViewport` _output_get 0)
        (`KismetSystemLibrary.Delay` 2.0)
        (`Widget.RemoveFromParent` _output_get)
        (set `self.Already Open` true)))))

(fn `ChangeSelectedDisc`
  (params (Right :type Boolean))
  (`self.SetSelectedDiscHighlight` false)
  (set `self.SelectedDiscIndex` (`KismetMathLibrary.Clamp` (+ (`self.SelectedDiscIndex`) (`KismetMathLibrary.SelectInt` 1 -1 Right)) 0 (`KismetArrayLibrary.Array_LastIndex` (`self.Disc`))))
  (`self.SetSelectedDiscHighlight` true))

(fn `EvaluateCombination`
  (returns (CombinationCorrect :type Boolean))
  (for (_array_element _array_index) (`self.Disc`)
    (if (`|EnumInequality` (`/Game/BPs/Chest/BP_NumberWheel.GetCurrentNumber` _array_element) (`|GetArrayItem` (`self.CorrectCode`) _array_index))
      (return false)))
  (return true))

(fn `GetSelectedDisc`
  (returns (Output :type "/Game/BPs/Chest/BP_NumberWheel Object Reference"))
  (return (`|GetArrayItem` (`self.Disc`) (`self.SelectedDiscIndex`))))

(fn `Interact`
  (params (PlayerCharacter :type "/Game/BPs/BP_FirstPersonCharacter Object Reference") (Pickup :type "/Game/BPs/Pickup/BP_Pickup Object Reference"))
  (returns (UsedUpPickup :type Boolean))
  (`parent.Interact` PlayerCharacter Pickup)
  (`self.SetSelectedDiscHighlight` true)
  (bind _returnvalue (`|CreateWidget` "/Game/BPs/Chest/BPW_ControllsLocks.BPW_ControllsLocks_C" (`GameplayStatics.GetPlayerController` 0)))
  (bind _output_get (set `self.BPW_Painting` _returnvalue))
  (`UserWidget.AddToViewport` _output_get 0)
  (return false))

(fn `SetSelectedDiscHighlight`
  (params (Enable :type Boolean))
  (`self.SetHighlight` Enable (`self.GetSelectedDisc`)))

(fn `UserConstructionScript`)