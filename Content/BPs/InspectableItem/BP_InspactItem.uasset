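; BP_InspactItem is an inspectable item that shows its text and emotion in a UI widget while the player inspects it.
; BeginPlay caches the item's starting transform and the first-person character.
; StartInspection adds a BPW_Inspectable widget built from the item's ItemText and EEmotion values and hides the character's crosshair.
; EndInspect restores the original transform, removes the widget and shows the crosshair again.
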(event `self.ReceiveBeginPlay`
  (set `self.StartTransform` (`self.GetTransform`))
  (bind _asbp_first_person_character (cast `/Game/BPs/BP_FirstPersonCharacter` (`GameplayStatics.GetPlayerCharacter` 0)))
  (set `self.As BP First Person Character` _asbp_first_person_character))

(event `StartInspection`
  (bind _returnvalue (`|CreateWidget` "/Game/BPs/InspectableItem/BPW_Inspectable.BPW_Inspectable_C" (`GameplayStatics.GetPlayerController` 0) (`self.Item Text`) (`self.EEmotion`)))
  (bind _output_get (set `self.InspectWidgetRef` _returnvalue))
  (`UserWidget.AddToViewport` _output_get 0)
  (`/Game/BPs/BP_FirstPersonCharacter.Show/Hide Crosshair` (`self.As BP First Person Character`) false))

(event `EndInspect`
  (`self.K2_SetActorTransform` (`self.StartTransform`))
  (`Widget.RemoveFromParent` (`self.InspectWidgetRef`))
  (`/Game/BPs/BP_FirstPersonCharacter.Show/Hide Crosshair` (`self.As BP First Person Character`) true))

(fn `UserConstructionScript`)