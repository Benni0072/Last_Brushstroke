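; Interactable puzzle in which the player selects and rotates three canvases, built on a parent that handles interaction and returning to the character.
; Interacting shows a controls widget and highlights the selected canvas.
; Input actions step the selection along the canvas array, clamped at both ends, and tell the selected canvas to rotate left or right.
; Exiting removes the widget, clears the highlight and resets the selection.
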(event `self.ReceiveBeginPlay`
  (`parent.ReceiveBeginPlay`)
  (set `self.Canvas` (`|MakeArray` (`self.BP_RotateCanvas`) (`self.BP_RotateCanvas1`) (`self.BP_RotateCanvas2`))))

(event `EnhancedInput|/Game/Inputs/InputActions/IA_ExitPuzzle`
  (params (ActionValue :type Boolean) (ElapsedSeconds :type "Float (double-precision)") (TriggeredSeconds :type "Float (double-precision)") (InputAction :type "InputAction Object Reference" :default "/Game/Inputs/InputActions/IA_ExitPuzzle.IA_ExitPuzzle"))
  (:`Triggered`
    (`Widget.RemoveFromParent` (`self.ControllWidget`))
    (`self.ReturnToCharacter`)))

(event `self.ReturnToCharacter`
  (`parent.ReturnToCharacter`)
  (`self.SetSelectetCanvasHighlight` false)
  (set `self.SelectedDiscIndex` 0))

(event `EnhancedInput|/Game/Inputs/InputActions/IA_RotateCanvasRight`
  (params (ActionValue :type Boolean) (ElapsedSeconds :type "Float (double-precision)") (TriggeredSeconds :type "Float (double-precision)") (InputAction :type "InputAction Object Reference" :default "/Game/Inputs/InputActions/IA_RotateCanvasRight.IA_RotateCanvasRight"))
  (:`Triggered`
    (`/Game/BPs/CanvasRotatePuzzle/BP_RotateCanvas.Rotate` (`self.GetSelectedCanvas`) false)))

(event `EnhancedInput|/Game/Inputs/InputActions/IA_RotateCanvasLeft`
  (params (ActionValue :type Boolean) (ElapsedSeconds :type "Float (double-precision)") (TriggeredSeconds :type "Float (double-precision)") (InputAction :type "InputAction Object Reference" :default "/Game/Inputs/InputActions/IA_RotateCanvasLeft.IA_RotateCanvasLeft"))
  (:`Triggered`
    (`/Game/BPs/CanvasRotatePuzzle/BP_RotateCanvas.Rotate` (`self.GetSelectedCanvas`) true)))

(event `EnhancedInput|/Game/Inputs/InputActions/IA_NavigateRight`
  (params (ActionValue :type Boolean) (ElapsedSeconds :type "Float (double-precision)") (TriggeredSeconds :type "Float (double-precision)") (InputAction :type "InputAction Object Reference" :default "/Game/Inputs/InputActions/IA_NavigateRight.IA_NavigateRight"))
  (:`Triggered`
    (`self.ChangeSelectedCanvas` true)))

(event `EnhancedInput|/Game/Inputs/InputActions/IA_NavigateLeft`
  (params (ActionValue :type Boolean) (ElapsedSeconds :type "Float (double-precision)") (TriggeredSeconds :type "Float (double-precision)") (InputAction :type "InputAction Object Reference" :default "/Game/Inputs/InputActions/IA_NavigateLeft.IA_NavigateLeft"))
  (:`Triggered`
    (`self.ChangeSelectedCanvas` false)))

(fn `ChangeSelectedCanvas`
  (params (Right :type Boolean))
  (`self.SetSelectetCanvasHighlight` false)
  (set `self.SelectedDiscIndex` (`KismetMathLibrary.Clamp` (+ (`self.SelectedDiscIndex`) (`KismetMathLibrary.SelectInt` 1 -1 Right)) 0 (`KismetArrayLibrary.Array_LastIndex` (`self.Canvas`))))
  (`self.SetSelectetCanvasHighlight` true))

(fn `GetSelectedCanvas`
  (returns (Output :type "/Game/BPs/CanvasRotatePuzzle/BP_RotateCanvas Object Reference"))
  (return (`|GetArrayItem` (`self.Canvas`) (`self.SelectedDiscIndex`))))

(fn `Interact`
  (params (PlayerCharacter :type "/Game/BPs/BP_FirstPersonCharacter Object Reference") (Pickup :type "/Game/BPs/Pickup/BP_Pickup Object Reference"))
  (returns (UsedUpPickup :type Boolean))
  (`parent.Interact` PlayerCharacter Pickup)
  (bind _returnvalue (`|CreateWidget` "/Game/BPs/CanvasRotatePuzzle/BPW_RotateCanvasCotrolls.BPW_RotateCanvasCotrolls_C" (`GameplayStatics.GetPlayerController` 0)))
  (bind _output_get (set `self.ControllWidget` _returnvalue))
  (`UserWidget.AddToViewport` _output_get 0)
  (`self.SetSelectetCanvasHighlight` true)
  (return false))

(fn `SetSelectetCanvasHighlight`
  (params (Enable :type Boolean))
  (`self.SetHighlight` Enable (`self.GetSelectedCanvas`)))

(fn `UserConstructionScript`)