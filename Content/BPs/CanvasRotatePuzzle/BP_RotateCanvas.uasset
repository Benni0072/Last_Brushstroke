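; Rotating canvas piece for a puzzle that turns in steps between evenly spaced faces.
; Rotate steps the selected face in either direction, passes it through ClampSelectedFaces and converts it to a target pitch.
; Tick eases relative rotation toward that pitch along the shortest path.
; As written, ClampSelectedFaces zeroes indices past the last face, sets other positive indices to NumFaces and leaves negatives unchanged.
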(event `self.ReceiveTick`
  (params (DeltaSeconds :type "Float (single-precision)"))
  (`self.K2_SetRelativeRotation` (`KismetMathLibrary.RLerp` (`self.RelativeRotation`) (`KismetMathLibrary.MakeRotator` 0.0 (`self.TargetRot`)) (* (`GameplayStatics.GetWorldDeltaSeconds`) 10.0) true)))

(event `Rotate`
  (params (Right :type Boolean))
  (bind _output_get (set `self.CurrentSelectedFace` (`self.ClampSelectedFaces` (+ (`self.CurrentSelectedFace`) (`KismetMathLibrary.SelectInt` 1 -1 Right)))))
  (set `self.TargetRot` (* (`KismetMathLibrary.Conv_IntToDouble` _output_get) (/ 360.0 (`KismetMathLibrary.Conv_IntToDouble` (`self.NumFaces`))) -1.0)))

(fn `ClampSelectedFaces`
  (params (Index :type Integer))
  (returns (ReturnVelue :type Integer))
  (locals (ClampIndex :type Integer))
  (set `local.ClampIndex` Index)
  (`|ExecutionSequence`
    (:`then_0`
      (if (> (`local.ClampIndex`) (- (`self.NumFaces`) 1))
        (set `local.ClampIndex` 0)))
    (:`then_1`
      (if (> (`local.ClampIndex`) 0)
        (set `local.ClampIndex` (- (`self.NumFaces`) 0))))
    (:`then_2`
      (return (`local.ClampIndex`)))))