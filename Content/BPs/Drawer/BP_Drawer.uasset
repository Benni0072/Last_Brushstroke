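; BP_Drawer is an interactable drawer that slides open and closed.
; Interact toggles Open and calls MoveDrawer, which plays or reverses the OpenClose timeline to lerp the Scene component along X from an offset based on Root's relative location.
; CanOpen acts as a busy lock until the timeline finishes, though Open still toggles on interactions during movement.
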(event `MoveDrawer`
  (bind (_relativelocation_x _relativelocation_y _relativelocation_z) (`KismetMathLibrary.BreakVector` (`SceneComponent.RelativeLocation` (`self.Root`))))
  (if (not (`self.CanOpen?`))
    (set `self.CanOpen?` true)
    (if (`self.Open?`)
      (set `self.Open?` true)
      (set `self.MoveDistance` 30.0)
      (set `self.StartLocation` (`KismetMathLibrary.MakeVector` _relativelocation_x _relativelocation_y _relativelocation_z))
      (set `self.EndLocation` (`KismetMathLibrary.MakeVector` (+ _relativelocation_x (`self.MoveDistance`)) _relativelocation_y _relativelocation_z))
      (bind (_direction _newtrack_0) (`Timeline|Open/Close` :!label _label)
        (:`Update`
          (`SceneComponent.K2_SetRelativeLocation` (`self.Scene`) (`KismetMathLibrary.VLerp` (`self.StartLocation`) (`self.EndLocation`) _newtrack_0) false false))
        (:`Finished`
          (set `self.CanOpen?` false)))
      (else
        (set `self.Open?` false)
        (set `self.MoveDistance` -30.0)
        (goto _label :!via `Reverse`)))))

(fn `Interact`
  (params (PlayerCharacter :type "/Game/BPs/BP_FirstPersonCharacter Object Reference") (Pickup :type "/Game/BPs/Pickup/BP_Pickup Object Reference"))
  (returns (UsedUpPickup :type Boolean))
  (set `self.PlayerCharacter` PlayerCharacter)
  (if (`self.Open?`)
    (set `self.Open?` false)
    (else
      (set `self.Open?` true)))
  (`self.MoveDrawer`)
  (return false))

(fn `UserConstructionScript`)