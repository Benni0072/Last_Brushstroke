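; Possessable keypad puzzle that opens a linked BP_Door when the correct code is entered.
; Navigation input moves a highlight across a wrapping three-column button grid, and Interact types, clears or confirms, using the TextRender display as the code buffer.
; A correct code blends to a camera, opens the door, returns to the character and disables possession.
; A wrong code clears the display and can briefly show an inspectable text widget.
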(event `self.ReceiveBeginPlay`
  (set `self.Buttons` (`|MakeArray` (`self.BP_KeypadButton`) (`self.BP_KeypadButton1`) (`self.BP_KeypadButton2`) (`self.BP_KeypadButton3`) (`self.BP_KeypadButton4`) (`self.BP_KeypadButton5`) (`self.BP_KeypadButton6`) (`self.BP_KeypadButton7`) (`self.BP_KeypadButton8`) (`self.BP_KeypadButtonCancle`) (`self.BP_KeypadButton10`) (`self.BP_KeypadButtonConfirm`)))
  (`self.ClearDisplay`))

(event `EnhancedInput|/Game/Inputs/InputActions/IA_ExitPuzzle`
  (params (ActionValue :type Boolean) (ElapsedSeconds :type "Float (double-precision)") (TriggeredSeconds :type "Float (double-precision)") (InputAction :type "InputAction Object Reference" :default "/Game/Inputs/InputActions/IA_ExitPuzzle.IA_ExitPuzzle"))
  (:`Triggered`
    (`self.ReturnToCharacter`)
    (`self.UpdateHighlightOfSelectedButton` false)))

(event `EnhancedInput|/Game/Inputs/InputActions/IA_NavigateRight`
  (params (ActionValue :type Boolean) (ElapsedSeconds :type "Float (double-precision)") (TriggeredSeconds :type "Float (double-precision)") (InputAction :type "InputAction Object Reference" :default "/Game/Inputs/InputActions/IA_NavigateRight.IA_NavigateRight"))
  (:`Triggered`
    (`self.NavigateButtons` 1)))

(event `EnhancedInput|/Game/Inputs/InputActions/IA_NavigateLeft`
  (params (ActionValue :type Boolean) (ElapsedSeconds :type "Float (double-precision)") (TriggeredSeconds :type "Float (double-precision)") (InputAction :type "InputAction Object Reference" :default "/Game/Inputs/InputActions/IA_NavigateLeft.IA_NavigateLeft"))
  (:`Triggered`
    (`self.NavigateButtons` -1)))

(event `EnhancedInput|/Game/Inputs/InputActions/IA_NavigateDown`
  (params (ActionValue :type Boolean) (ElapsedSeconds :type "Float (double-precision)") (TriggeredSeconds :type "Float (double-precision)") (InputAction :type "InputAction Object Reference" :default "/Game/Inputs/InputActions/IA_NavigateDown.IA_NavigateDown"))
  (:`Triggered`
    (`self.NavigateButtons` 3)))

(event `EnhancedInput|/Game/Inputs/InputActions/IA_NavigateUp`
  (params (ActionValue :type Boolean) (ElapsedSeconds :type "Float (double-precision)") (TriggeredSeconds :type "Float (double-precision)") (InputAction :type "InputAction Object Reference" :default "/Game/Inputs/InputActions/IA_NavigateUp.IA_NavigateUp"))
  (:`Triggered`
    (`self.NavigateButtons` -3)))

(event `EnhancedInput|/Game/Inputs/InputActions/IA_Interact`
  (params (ActionValue :type Boolean) (ElapsedSeconds :type "Float (double-precision)") (TriggeredSeconds :type "Float (double-precision)") (InputAction :type "InputAction Object Reference" :default "/Game/Inputs/InputActions/IA_Interact.IA_Interact"))
  (:`Triggered`
    (`GameplayStatics.PlaySound2D` "/Game/Sound/SFX/Keypad/KeypadTasten.KeypadTasten" 1.0 1.0 0.0 null null)
    (if (== (`self.GetSelectedButton`) (`self.BP_KeypadButtonConfirm`))
      (if (`self.IsCodeCorrect`)
        (`GameplayStatics.PlaySound2D` "/Game/Sound/SFX/Keypad/correct-Pin.correct-Pin" 1.0 1.0 0.0 null null)
        (`PlayerController.SetViewTargetWithBlend` (`GameplayStatics.GetPlayerController` 0) (`self.CameraActor`) (`self.SmoothPossessDuartion`) "VTBlend_EaseInOut" (`self.Possess Blend Exp`) false)
        (`KismetSystemLibrary.Delay` (`self.SmoothPossessDuartion`))
        (bind _asbp_door (cast `/Game/BPs/Keypad/BP_Door` (`self.Actor`)))
        (`/Game/BPs/Keypad/BP_Door.OpenDoor` _asbp_door)
        (`KismetSystemLibrary.Delay` 3.1)
        (`self.ReturnToCharacter`)
        (`self.UpdateHighlightOfSelectedButton` false)
        (set `self.CanBePossessed?` false)
        (else
          (`GameplayStatics.PlaySound2D` "/Game/Sound/SFX/Keypad/wrong-Pin.wrong-Pin" 1.0 1.0 0.0 null null)
          (`self.ClearDisplay`)
          (if (`self.AlreadyOpen`)
            (set `self.AlreadyOpen` false)
            (bind _returnvalue (`|CreateWidget` "/Game/BPs/InspectableItem/BPW_Inspectable.BPW_Inspectable_C" (`GameplayStatics.GetPlayerController` 0) (`self.Item Text`) (`self.EEmotion`)))
            (bind _output_get (set `self.WBP_Inspectable` _returnvalue))
            (`UserWidget.AddToViewport` _output_get 0)
            (`KismetSystemLibrary.Delay` 2.0)
            (`Widget.RemoveFromParent` _output_get)
            (set `self.AlreadyOpen` true))))
      (elif (== (`self.GetSelectedButton`) (`self.BP_KeypadButtonCancle`))
        (`self.ClearDisplay`)
        (elif (not (`self.IsCodeComplet`))
          (`self.AddToDisplay` (`/Game/BPs/Keypad/BP_KeypadButton.ButtonLabel` (`self.GetSelectedButton`))))))))

(fn `AddToDisplay`
  (params (B :type String))
  (bind _textrender (`self.TextRender`))
  (`TextRenderComponent.K2_SetText` _textrender (`KismetTextLibrary.Conv_StringToText` (`KismetStringLibrary.Concat_StrStr` (`KismetTextLibrary.Conv_TextToString` (`TextRenderComponent.Text` _textrender)) B))))

(fn `ClearDisplay`
  (`TextRenderComponent.K2_SetText` (`self.TextRender`) (`KismetTextLibrary.Conv_StringToText` "")))

(fn `GetSelectedButton`
  (returns (Output :type "/Game/BPs/Keypad/BP_KeypadButton Object Reference"))
  (return (`|GetArrayItem` (`self.Buttons`) (`self.CurrentButtonIndex`))))

(fn `Interact`
  (params (PlayerCharacter :type "/Game/BPs/BP_FirstPersonCharacter Object Reference") (Pickup :type "/Game/BPs/Pickup/BP_Pickup Object Reference"))
  (returns (UsedUpPickup :type Boolean))
  (`parent.Interact` PlayerCharacter Pickup)
  (if (`self.CanBePossessed?`)
    (`self.UpdateHighlightOfSelectedButton` true)
    (return false)))

(fn `IsCodeComplet`
  (returns (ReturnValue :type Boolean))
  (return (== (`KismetStringLibrary.Len` (`KismetTextLibrary.Conv_TextToString` (`TextRenderComponent.Text` (`self.TextRender`)))) (`KismetStringLibrary.Len` (`self.CorrectCode`)))))

(fn `IsCodeCorrect`
  (returns (ReturnValue :type Boolean))
  (return (`KismetStringLibrary.EqualEqual_StrStr` (`KismetTextLibrary.Conv_TextToString` (`TextRenderComponent.Text` (`self.TextRender`))) (`self.CorrectCode`))))

(fn `NavigateButtons`
  (params (Direction :type Integer))
  (`self.UpdateHighlightOfSelectedButton` false)
  (set `self.CurrentButtonIndex` (+ (`self.CurrentButtonIndex`) Direction))
  (`|ExecutionSequence`
    (:`then_0`
      (if (> (`self.CurrentButtonIndex`) (`KismetArrayLibrary.Array_LastIndex` (`self.Buttons`)))
        (set `self.CurrentButtonIndex` (- (`self.CurrentButtonIndex`) (`KismetArrayLibrary.Array_Length` (`self.Buttons`))))))
    (:`then_1`
      (if (< (`self.CurrentButtonIndex`) 0)
        (set `self.CurrentButtonIndex` (+ (`self.CurrentButtonIndex`) (`KismetArrayLibrary.Array_Length` (`self.Buttons`))))))
    (:`then_2`
      (`self.UpdateHighlightOfSelectedButton` true))))

(fn `UpdateHighlightOfSelectedButton`
  (params (Enable :type Boolean))
  (`MeshComponent.SetOverlayMaterial` (`self.GetSelectedButton`) (select `bool` Enable :`true` "/Game/Material/highlight/MM_Highlight.MM_Highlight" :!type "MaterialInterface Object Reference")))

(fn `UserConstructionScript`)