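; BP_Door is a door actor, filed with the keypad Blueprints, that swings open when its OpenDoor event is called.
; After a short delay, a timeline drives the root's yaw scaled by OpenAgnle and the handle's roll scaled by Rotation.
; A DoOnce on the timeline update plays the wooden handle sound a single time, followed by a delay that leads to nothing.
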(event `OpenDoor`
  (`KismetSystemLibrary.Delay` 0.2)
  (bind (_direction _newtrack_0 _handle) (`Timeline|Open Door`)
    (:`Update`
      (`SceneComponent.K2_SetRelativeRotation` (`self.DefaultSceneRoot`) (`KismetMathLibrary.MakeRotator` 0.0 0.0 (* _newtrack_0 (`self.OpenAgnle`))) false false)
      (`SceneComponent.K2_SetRelativeRotation` (`self. Handle`) (`KismetMathLibrary.MakeRotator` (* _handle (`self.Rotation`))) false false)
      (`/Engine/EditorBlueprintResources/StandardMacros.DoOnce` false
        (:`Completed`
          (`GameplayStatics.PlaySound2D` "/Game/Sound/SFX/wooden-door-handle.wooden-door-handle" 1.0 1.0 0.0 null null)
          (`KismetSystemLibrary.Delay` 2.8))))))

(fn `UserConstructionScript`)