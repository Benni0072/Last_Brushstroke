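; BP_PickupTarget is a puzzle receptacle that accepts one desired pickup class, attaches it to a target transform, and can then be rotated.
; Later interactions roll the root by one face of NumFaces and increment a counter when rotation is allowed.
; If correct rotation is required, a count of exactly three shows the WBP_Comic2 widget and destroys ActorFog.
; A yaw-based RotateStatue variant exists but is not called here.
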(fn `Interact`
  (params (PlayerCharacter :type "/Game/BPs/BP_FirstPersonCharacter Object Reference") (Pickup :type "/Game/BPs/Pickup/BP_Pickup Object Reference"))
  (returns (UsedUpPickup :type Boolean))
  (if (`self.HasRecivedPickup`)
    (if (`self.CanBeRotated`)
      (`self.Rotate`)
      (if (`self.MustBeRotatedCorrectly`)
        (if (== (`self.Rotation`) 3.0)
          (bind _returnvalue (`|CreateWidget` "/Game/UI/Comics/WBP_Comic2.WBP_Comic2_C" (`GameplayStatics.GetPlayerController` 0)))
          (bind _output_get (set `self.WBP_Comic2` _returnvalue))
          (`UserWidget.AddToViewport` _output_get 0)
          (`self.K2_DestroyActor` (`self.ActorFog`)))))
    (else
      (`/Engine/EditorBlueprintResources/StandardMacros.IsValid` Pickup
        (:`Is Valid`
          (if (== (`GameplayStatics.GetObjectClass` Pickup) (`self.DisiredPickup`))
            (`/Game/BPs/Pickup/BP_Pickup.AttachTo` Pickup (`self.TargetTransform`))
            (set `self.HasRecivedPickup` true)
            (return true)
            (else
              (return false))))))))

(fn `Rotate`
  (`SceneComponent.K2_AddRelativeRotation` (`self.DefaultSceneRoot`) (`KismetMathLibrary.MakeRotator` (/ 360.0 (`KismetMathLibrary.Conv_IntToDouble` (`self.NumFaces`)))) false false)
  (set `self.Rotation` (+ 1.0 (`self.Rotation`))))

(fn `RotateStatue`
  (`SceneComponent.K2_AddRelativeRotation` (`self.DefaultSceneRoot`) (`KismetMathLibrary.MakeRotator` 0.0 0.0 (/ 360.0 (`KismetMathLibrary.Conv_IntToDouble` (`self.NumFaces`)))) false false)
  (set `self.Rotation` (+ 1.0 (`self.Rotation`))))

(fn `UserConstructionScript`)