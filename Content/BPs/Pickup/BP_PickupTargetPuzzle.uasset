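; BP_PickupTargetPuzzle is an interactable puzzle target that rotates on use and can reward reaching the correct orientation.
; Interact calls Rotate, then, if MustBeRotatedCorrectly is set, checks Rotation against one hardcoded value.
; On a match it shows the WBP_Comic2 widget on screen and destroys the referenced ActorFog.
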(fn `Interact`
  (params (PlayerCharacter :type "/Game/BPs/BP_FirstPersonCharacter Object Reference") (Pickup :type "/Game/BPs/Pickup/BP_Pickup Object Reference"))
  (returns (UsedUpPickup :type Boolean))
  (`self.Rotate`)
  (if (`self.MustBeRotatedCorrectly`)
    (if (== (`self.Rotation`) 3.0)
      (bind _returnvalue (`|CreateWidget` "/Game/UI/Comics/WBP_Comic2.WBP_Comic2_C" (`GameplayStatics.GetPlayerController` 0)))
      (bind _output_get (set `self.WBP_Comic2` _returnvalue))
      (`UserWidget.AddToViewport` _output_get 0)
      (`self.K2_DestroyActor` (`self.ActorFog`)))))

(fn `UserConstructionScript`
  (`parent.UserConstructionScript`))