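; BP_Computer is an interactable computer in the printing puzzle that opens an on-screen computer interface for the player.
; Interact creates a WBP_Computerscreen widget, hands it a back-reference to the computer and its Referenz variable, then switches to UI-only input with a visible cursor.
; The CloseComputer event removes the widget, restores game-only input and hides the cursor.
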(event `CloseComputer`
  (bind _returnvalue (`GameplayStatics.GetPlayerController` 0))
  (`WidgetBlueprintLibrary.SetInputMode_GameOnly` _returnvalue)
  (`Widget.RemoveFromParent` (`self.BPW Computerscreen`))
  (set `PlayerController.bShowMouseCursor` false _returnvalue))

(fn `Interact`
  (params (PlayerCharacter :type "/Game/BPs/BP_FirstPersonCharacter Object Reference") (Pickup :type "/Game/BPs/Pickup/BP_Pickup Object Reference"))
  (returns (UsedUpPickup :type Boolean))
  (bind _returnvalue (`GameplayStatics.GetPlayerController` 0))
  (`WidgetBlueprintLibrary.SetInputMode_UIOnlyEx` _returnvalue null)
  (bind _returnvalue_2 (`|CreateWidget` "/Game/BPs/PrintingPuzzle/WBP_Computerscreen.WBP_Computerscreen_C" _returnvalue))
  (bind _output_get (set `self.BPW Computerscreen` _returnvalue_2))
  (set `/Game/BPs/PrintingPuzzle/WBP_Computerscreen.BP Computer` self _output_get)
  (set `PlayerController.bShowMouseCursor` true (`GameplayStatics.GetPlayerController` 0))
  (`UserWidget.AddToViewport` _output_get 0)
  (set `/Game/BPs/PrintingPuzzle/WBP_Computerscreen.Referenz` (`self.Referenz`) (`self.BPW Computerscreen`))
  (return false))

(fn `UserConstructionScript`)