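; An interactable pawn base for puzzles that the player can possess from the first-person character and later leave.
; Interact stores the character and, if possession is allowed, starts GetPossessed, which hides the crosshair, blends the view to this pawn, then possesses it.
; ReturnToCharacter reverses this, with both directions swapping Enhanced Input mapping contexts and delaying possession until the camera blend finishes.
; SetHighlight toggles an overlay material on a given mesh.
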(event `GetPossessed`
  (`/Game/BPs/BP_FirstPersonCharacter.Show/Hide Crosshair` (`self.FirstPersonCharacter`) false)
  (`EnhancedInputSubsystemInterface.RemoveMappingContext` (pcsubsystem `EnhancedInputLocalPlayerSubsystem` (`GameplayStatics.GetPlayerController` 0)) (`self.Player Mapping Context`) (struct))
  (`PlayerController.SetViewTargetWithBlend` (`GameplayStatics.GetPlayerController` 0) self (`self.SmoothPossessDuration`) (`self.PossessionBlendFunction`) (`self.PossesssBlendExponent`) false)
  (`KismetSystemLibrary.Delay` (`self.SmoothPossessDuration`))
  (`Controller.Possess` (`GameplayStatics.GetPlayerController` 0) self)
  (`EnhancedInputSubsystemInterface.AddMappingContext` (pcsubsystem `EnhancedInputLocalPlayerSubsystem` (`GameplayStatics.GetPlayerController` 0)) (`self.PuzzleMapping Context`) 0 (struct)))

(event `ReturnToCharacter`
  (`EnhancedInputSubsystemInterface.RemoveMappingContext` (pcsubsystem `EnhancedInputLocalPlayerSubsystem` (`GameplayStatics.GetPlayerController` 0)) (`self.PuzzleMapping Context`) (struct))
  (`PlayerController.SetViewTargetWithBlend` (`GameplayStatics.GetPlayerController` 0) (`self.FirstPersonCharacter`) (`self.SmoothPossessDuration`) (`self.PossessionBlendFunction`) (`self.PossesssBlendExponent`) false)
  (`KismetSystemLibrary.Delay` (`self.SmoothPossessDuration`))
  (`EnhancedInputSubsystemInterface.AddMappingContext` (pcsubsystem `EnhancedInputLocalPlayerSubsystem` (`GameplayStatics.GetPlayerController` 0)) (`self.Player Mapping Context`) 0 (struct))
  (`Controller.Possess` (`GameplayStatics.GetPlayerController` 0) (`self.FirstPersonCharacter`))
  (`WidgetBlueprintLibrary.SetInputMode_GameOnly` (`GameplayStatics.GetPlayerController` 0))
  (`/Game/BPs/BP_FirstPersonCharacter.Show/Hide Crosshair` (`self.FirstPersonCharacter`) true))

(fn `Interact`
  (params (PlayerCharacter :type "/Game/BPs/BP_FirstPersonCharacter Object Reference") (Pickup :type "/Game/BPs/Pickup/BP_Pickup Object Reference"))
  (returns (UsedUpPickup :type Boolean))
  (set `self.FirstPersonCharacter` PlayerCharacter)
  (if (`self.CanBePossessed?`)
    (`self.GetPossessed`)
    (return false)))

(fn `SetHighlight`
  (params (Enable :type Boolean) (MeshComponent :type "MeshComponent Object Reference"))
  (`MeshComponent.SetOverlayMaterial` MeshComponent (select `bool` Enable :`true` "/Game/Material/highlight/MI_Highlight.MI_Highlight" :!type "MaterialInterface Object Reference")))

(fn `UserConstructionScript`)