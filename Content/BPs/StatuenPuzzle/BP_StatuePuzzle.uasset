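; BP_StatuePuzzle is an interactable puzzle in which the player rotates a statue.
; Interacting runs the parent logic and shows a rotate-controls widget; the exit input removes it and returns to the character.
; Left and right rotate inputs turn the selected entry in the Canvas array, filled with a single statue on BeginPlay.
; A selection function steps a clamped index and moves the highlight, but nothing in this graph calls it.
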(event `self.ReceiveBeginPlay`
  (`parent.ReceiveBeginPlay`)
  (set `self.Canvas` (`|MakeArray` (`self.BP_Statue`))))

(event `EnhancedInput|/Game/Inputs/InputActions/IA_ExitPuzzle`
  (params (ActionValue :type Boolean) (ElapsedSeconds :type "Float (double-precision)") (TriggeredSeconds :type "Float (double-precision)") (InputAction :type "InputAction Object Reference" :default "/Game/Inputs/InputActions/IA_ExitPuzzle.IA_ExitPuzzle"))
  (:`Triggered`
    (`Widget.RemoveFromParent` (`self.RotateControllWidget`))
    (`self.ReturnToCharacter`)))

(event `self.ReturnToCharacter`
  (`parent.ReturnToCharacter`))

(event `EnhancedInput|/Game/Inputs/InputActions/IA_RotateCanvasRight`
  (params (ActionValue :type Boolean) (ElapsedSeconds :type "Float (double-precision)") (TriggeredSeconds :type "Float (double-precision)") (InputAction :type "InputAction Object Reference" :default "/Game/Inputs/InputActions/IA_RotateCanvasRight.IA_RotateCanvasRight"))
  (:`Triggered`
    (`/Game/BPs/StatuenPuzzle/BP_Statue.Rotate` (`self.GetSelectedStatue`) false)))

(event `EnhancedInput|/Game/Inputs/InputActions/IA_RotateCanvasLeft`
  (params (ActionValue :type Boolean) (ElapsedSeconds :type "Float (double-precision)") (TriggeredSeconds :type "Float (double-precision)") (InputAction :type "InputAction Object Reference" :default "/Game/Inputs/InputActions/IA_RotateCanvasLeft.IA_RotateCanvasLeft"))
  (:`Triggered`
    (`/Game/BPs/StatuenPuzzle/BP_Statue.Rotate` (`self.GetSelectedStatue`) true)))

(fn `ChangeSelectedCanvas`
  (params (Right :type Boolean))
  (`self.SetSelectetCanvasHighlight` false)
  (set `self.SelectedDiscIndex` (`KismetMathLibrary.Clamp` (+ (`self.SelectedDiscIndex`) (`KismetMathLibrary.SelectInt` 1 -1 Right)) 0 (`KismetArrayLibrary.Array_LastIndex` (`self.Canvas`))))
  (`self.SetSelectetCanvasHighlight` true))

(fn `GetSelectedStatue`
  (returns (Output :type "/Game/BPs/StatuenPuzzle/BP_Statue Object Reference"))
  (return (`|GetArrayItem` (`self.Canvas`) (`self.SelectedDiscIndex`))))

(fn `Interact`
  (params (PlayerCharacter :type "/Game/BPs/BP_FirstPersonCharacter Object Reference") (Pickup :type "/Game/BPs/Pickup/BP_Pickup Object Reference"))
  (returns (UsedUpPickup :type Boolean))
  (`parent.Interact` PlayerCharacter Pickup)
  (bind _returnvalue (`|CreateWidget` "/Game/BPs/StatuenPuzzle/BPW_RotateControlls.BPW_RotateControlls_C" (`GameplayStatics.GetPlayerController` 0)))
  (bind _output_get (set `self.RotateControllWidget` _returnvalue))
  (`UserWidget.AddToViewport` _output_get 0)
  (return false))

(fn `SetSelectetCanvasHighlight`
  (params (Enable :type Boolean))
  (`self.SetHighlight` Enable (`self.GetSelectedStatue`)))

(fn `UserConstructionScript`)